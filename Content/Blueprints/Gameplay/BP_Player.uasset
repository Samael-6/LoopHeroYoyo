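; Player character with Enhanced Input walking, mouse-style look and an endurance-limited sprint.
; Sprint doubles walk speed on start and halves it on release, draining endurance while held.
; Tick regenerates endurance when not running, flagging the player tired below a threshold to block new sprints.
; Exhaustion ends the sprint through a DoOnce that Tick re-arms while running, restoring speed and printing it.
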(event Input|EnhancedActionEvents|EnhancedInputActionIA_Walk
  (params (ActionValue :type Vector%202D%20Structure) (ElapsedSeconds :type Float%20%28double-precision%29) (TriggeredSeconds :type Float%20%28double-precision%29) (InputAction :type Input%20Action%20Object%20Reference :default "/Game/Blueprints/Inputs/IA_Walk.IA_Walk"))
  (bind (_x _y) (Math|Vector2D|BreakVector2D ActionValue))
  (bind _returnvalue (Pawn|GetControlRotation :!class /Script/Engine.Pawn))
  (Pawn|Input|AddMovementInput (Math|Vector|GetRightVector (Math|Rotator|MakeRotator (.roll _returnvalue) 0.0 (.yaw _returnvalue))) _x false)
  (Pawn|Input|AddMovementInput (Math|Vector|GetForwardVector (Math|Rotator|MakeRotator 0.0 0.0 (.yaw (Pawn|GetControlRotation :!class /Script/Engine.Pawn)))) _y false))

(event Input|EnhancedActionEvents|EnhancedInputActionIA_Look
  (params (ActionValue :type Vector%202D%20Structure) (ElapsedSeconds :type Float%20%28double-precision%29) (TriggeredSeconds :type Float%20%28double-precision%29) (InputAction :type Input%20Action%20Object%20Reference :default "/Game/Blueprints/Inputs/IA_Look.IA_Look"))
  (Pawn|Input|AddControllerYawInput (.x ActionValue))
  (Pawn|Input|AddControllerPitchInput (* (.y ActionValue) -1.0)))

(event Input|EnhancedActionEvents|EnhancedInputActionIA_Sprint
  (params (ActionValue :type Boolean) (ElapsedSeconds :type Float%20%28double-precision%29) (TriggeredSeconds :type Float%20%28double-precision%29) (InputAction :type Input%20Action%20Object%20Reference :default "/Game/Blueprints/Inputs/IA_Sprint.IA_Sprint"))
  (bind _charactermovement (Variables|Character|GetCharacterMovement))
  (bind _charactermovement_2 (Variables|Character|GetCharacterMovement))
  (bind _charactermovement_3 (Variables|Character|GetCharacterMovement))
  (:Triggered
    (if (or (<= (Variables|Default|GetEndurance) 0.0) (Variables|Default|GetIsTired))
      (Utilities|FlowControl|DoOnce false
        (:Completed
          (Variables|Default|SetIsRunning false)
          (Variables|Default|SetIsTired true)
          (bind _output_get (Variables|/Script/Engine.CharacterMovementComponent|SetMaxWalkSpeed _charactermovement (/ (Variables|/Script/Engine.CharacterMovementComponent|GetMaxWalkSpeed _charactermovement) 2.0)))
          (Development|PrintString (Utilities|String|ToString(Float) _output_get) true true "(R=0.154906,G=1.000000,B=0.000000,A=1.000000)")))
      (else
        (Variables|Default|SetEndurance (Math|Float|Clamp(Float) (- (Variables|Default|GetEndurance) (* ElapsedSeconds 0.5)) 0.0 1e+02)))))
  (:Started
    (if (not (Variables|Default|GetIsTired))
      (Variables|Default|SetIsRunning true)
      (Variables|/Script/Engine.CharacterMovementComponent|SetMaxWalkSpeed _charactermovement_3 (* (Variables|/Script/Engine.CharacterMovementComponent|GetMaxWalkSpeed _charactermovement_3) 2.0))))
  (:Completed
    (if (Variables|Default|GetIsRunning)
      (Variables|/Script/Engine.CharacterMovementComponent|SetMaxWalkSpeed _charactermovement_2 (/ (Variables|/Script/Engine.CharacterMovementComponent|GetMaxWalkSpeed _charactermovement_2) 2.0))
      (Variables|Default|SetIsRunning false))))

(event EventBeginPlay)

(event Collision|EventActorBeginOverlap
  (params (OtherActor :type Actor%20Object%20Reference)))

(event EventTick
  (params (DeltaSeconds :type Float%20%28single-precision%29))
  (bind _charactermovement (Variables|Character|GetCharacterMovement))
  (if (Variables|Default|GetIsRunning)
    (Utilities|FlowControl|DoOnce false) ; enters at Reset
    (else
      (bind _output_get (Variables|Default|SetEndurance (Math|Float|Clamp(Float) (+ (* DeltaSeconds 1e+01) (Variables|Default|GetEndurance)) 0.0 1e+02)))
      (Variables|Default|SetIsTired (< _output_get 3e+01)))))

(fn ConstructionScript)