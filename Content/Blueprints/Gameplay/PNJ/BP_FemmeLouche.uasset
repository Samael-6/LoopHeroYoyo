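; Shady woman NPC (FemmeLouche) that talks to the player and can send them to board cell 5 once.
; Activate feeds the current BPCDialogueComponent row to the pawn's dialogue widget, disabling help and jumping to row 5 if IsSuperSword is set.
; Update advances rows until the dialogue ends, then closes it, moves the pawn and activates that cell if CanHelp.
; Afterwards CanHelp is off and later conversations start at row 5.
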(event EventBeginPlay
  (|CallParentFunction) ; This node is disabled and will not be called.\nDrag off pins to build functionality.
)

(event Collision|EventActorBeginOverlap
  (params (OtherActor :type Actor%20Object%20Reference))
  (|CallParentFunction OtherActor) ; This node is disabled and will not be called.\nDrag off pins to build functionality.
)

(event EventTick
  (params (DeltaSeconds :type Float%20%28single-precision%29))
  (|CallParentFunction DeltaSeconds) ; This node is disabled and will not be called.\nDrag off pins to build functionality.
)

(event EventActivate
  (params (Pawn :type BP%20Pawn%20Object%20Reference))
  (bind _wbp_dialogue (Variables|/Game/Blueprints/Gameplay/BP_Pawn.BP_Pawn_C|GetWBP_Dialogue Pawn))
  (bind _bpc_dialoguecomponent (Variables|Default|GetBPC_DialogueComponent))
  (if (Variables|/Game/Blueprints/Gameplay/BP_Pawn.BP_Pawn_C|GetIsSuperSword Pawn)
    (Variables|Default|SetCanHelp false)
    (Variables|/Game/Blueprints/Global/BPC_DialogueComponent.BPC_DialogueComponent_C|SetCurrentRowNumber _bpc_dialoguecomponent 5))
  (Default|GetCurrentDialogueRowData _bpc_dialoguecomponent)
  (bind _charactername (Default|GetCharacterfromCurrentRow _bpc_dialoguecomponent))
  (bind _dialoguelong (Default|GetDialogueLongfromCurrentRow _bpc_dialoguecomponent))
  (Default|UpdateDialogue _wbp_dialogue _charactername _dialoguelong)
  (Default|StartDialogue _wbp_dialogue (Variables|/Game/Blueprints/Gameplay/BP_Pawn.BP_Pawn_C|GetDice Pawn)))

(event EventUpdate
  (params (Pawn :type BP%20Pawn%20Object%20Reference))
  (bind _bpc_dialoguecomponent (Variables|Default|GetBPC_DialogueComponent))
  (bind _isdialoguefinished (Default|IsDialogueFinished (Variables|Default|GetBPC_DialogueComponent)))
  (if _isdialoguefinished
    (Default|ExitDialogue (Variables|/Game/Blueprints/Gameplay/BP_Pawn.BP_Pawn_C|GetWBP_Dialogue Pawn))
    (if (Variables|Default|GetCanHelp)
      (Variables|/Game/Blueprints/Global/BP_LoopGameInstance.BP_LoopGameInstance_C|SetCellNumber (Variables|/Game/Blueprints/Gameplay/BP_Pawn.BP_Pawn_C|GetBP_LoopGameInstance Pawn) 5)
      (Default|MovetoCell Pawn)
      (Default|ActivateCell Pawn)
      (Variables|Default|SetCanHelp false))
    (Variables|/Game/Blueprints/Global/BPC_DialogueComponent.BPC_DialogueComponent_C|SetCurrentRowNumber (Variables|Default|GetBPC_DialogueComponent) 5)
    (else
      (Default|ReadNextRow _bpc_dialoguecomponent)
      (bind _charactername (Default|GetCharacterfromCurrentRow _bpc_dialoguecomponent))
      (bind _dialoguelong (Default|GetDialogueLongfromCurrentRow _bpc_dialoguecomponent))
      (Default|UpdateDialogue (Variables|/Game/Blueprints/Gameplay/BP_Pawn.BP_Pawn_C|GetWBP_Dialogue Pawn) _charactername _dialoguelong))))

(fn ConstructionScript
  (|CallParentFunction))