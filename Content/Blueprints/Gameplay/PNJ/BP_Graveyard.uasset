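; BP_Graveyard is a graveyard actor that grants the super sword upgrade to a pawn when activated.
; Its Activate event sets IsSuperSword on the pawn, acting only if that flag is not already set.
; It then shows a WBP_NotificationSword widget, plays its Fade animation, and removes it after a short delay.
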(event EventBeginPlay
  (|CallParentFunction) ; This node is disabled and will not be called.\nDrag off pins to build functionality.
)

(event Collision|EventActorBeginOverlap
  (params (OtherActor :type Actor%20Object%20Reference))
  (|CallParentFunction OtherActor) ; This node is disabled and will not be called.\nDrag off pins to build functionality.
)

(event EventTick
  (params (DeltaSeconds :type Float%20%28single-precision%29))
  (|CallParentFunction DeltaSeconds) ; This node is disabled and will not be called.\nDrag off pins to build functionality.
)

(event EventActivate
  (params (Pawn :type BP%20Pawn%20Object%20Reference))
  (if (not (Variables|/Game/Blueprints/Gameplay/BP_Pawn.BP_Pawn_C|GetIsSuperSword Pawn))
    (Variables|/Game/Blueprints/Gameplay/BP_Pawn.BP_Pawn_C|SetIsSuperSword Pawn true)
    (bind _returnvalue (UserInterface|CreateWidget "/Game/Blueprints/HUD/WBP_NotificationSword.WBP_NotificationSword_C"))
    (UserInterface|Viewport|AddtoViewport _returnvalue 0)
    (UserInterface|Animation|PlayAnimation _returnvalue (Variables|/Game/Blueprints/HUD/WBP_NotificationSword.WBP_NotificationSword_C|GetFade _returnvalue) 0.0 1 "Forward" 1.0 false)
    (Utilities|FlowControl|Delay 0.5)
    (Widget|RemovefromParent _returnvalue)))

(fn ConstructionScript
  (|CallParentFunction))