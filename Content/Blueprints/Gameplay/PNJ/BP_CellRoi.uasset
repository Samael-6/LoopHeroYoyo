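; BP_CellRoi is an NPC Blueprint that runs a branching dialogue through the interacting pawn's dialogue widget.
; Activate reads the current row from BPCDialogueComponent, shows speaker and line, then starts the dialogue with the pawn's Dice.
; Update advances to the next row or exits when the dialogue is finished.
; At a choice, it hands itself to the widget and adds one button per option, each carrying a row number.
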(event EventBeginPlay
  (|CallParentFunction) ; This node is disabled and will not be called.\nDrag off pins to build functionality.
)

(event Collision|EventActorBeginOverlap
  (params (OtherActor :type Actor%20Object%20Reference))
  (|CallParentFunction OtherActor) ; This node is disabled and will not be called.\nDrag off pins to build functionality.
)

(event EventTick
  (params (DeltaSeconds :type Float%20%28single-precision%29))
  (|CallParentFunction DeltaSeconds) ; This node is disabled and will not be called.\nDrag off pins to build functionality.
)

(event EventActivate
  (params (Pawn :type BP%20Pawn%20Object%20Reference))
  (bind _wbp_dialogue (Variables|/Game/Blueprints/Gameplay/BP_Pawn.BP_Pawn_C|GetWBP_Dialogue Pawn))
  (bind _bpc_dialoguecomponent (Variables|Default|GetBPC_DialogueComponent))
  (Default|GetCurrentDialogueRowData _bpc_dialoguecomponent)
  (bind _charactername (Default|GetCharacterfromCurrentRow _bpc_dialoguecomponent))
  (bind _dialoguelong (Default|GetDialogueLongfromCurrentRow _bpc_dialoguecomponent))
  (Default|UpdateDialogue _wbp_dialogue _charactername _dialoguelong)
  (Default|StartDialogue _wbp_dialogue (Variables|/Game/Blueprints/Gameplay/BP_Pawn.BP_Pawn_C|GetDice Pawn)))

(event EventUpdate
  (params (Pawn :type BP%20Pawn%20Object%20Reference))
  (bind _wbp_dialogue (Variables|/Game/Blueprints/Gameplay/BP_Pawn.BP_Pawn_C|GetWBP_Dialogue Pawn))
  (bind _bpc_dialoguecomponent (Variables|Default|GetBPC_DialogueComponent))
  (bind _bpc_dialoguecomponent_2 (Variables|Default|GetBPC_DialogueComponent))
  (bind _bpc_dialoguecomponent_3 (Variables|Default|GetBPC_DialogueComponent))
  (bind _ischoicenext (Default|IsChoiceNext _bpc_dialoguecomponent))
  (if _ischoicenext
    (Variables|/Game/Blueprints/HUD/WBP_DialogueUI.WBP_DialogueUI_C|SetBP_Cell _wbp_dialogue self)
    (for _index (range 0 (- (Variables|/Game/Blueprints/Global/BPC_DialogueComponent.BPC_DialogueComponent_C|GetNumberChoice _bpc_dialoguecomponent_2) 1))
      (Default|ReadNextRow _bpc_dialoguecomponent_2)
      (bind _dialoguelong (Default|GetDialogueLongfromCurrentRow _bpc_dialoguecomponent_2))
      (bind _nextrownumber (Default|GetNewRowNumber _bpc_dialoguecomponent_2))
      (Default|AddButton _wbp_dialogue _dialoguelong _nextrownumber))
    (Default|StartChoice _wbp_dialogue)
    (Variables|/Game/Blueprints/Global/BPC_DialogueComponent.BPC_DialogueComponent_C|SetNumberChoice _bpc_dialoguecomponent_2 0)
    (else
      (bind _isdialoguefinished (Default|IsDialogueFinished _bpc_dialoguecomponent))
      (if _isdialoguefinished
        (Default|ExitDialogue _wbp_dialogue)
        (else
          (Default|ReadNextRow _bpc_dialoguecomponent_3)
          (bind _charactername (Default|GetCharacterfromCurrentRow _bpc_dialoguecomponent_3))
          (bind _dialoguelong_2 (Default|GetDialogueLongfromCurrentRow _bpc_dialoguecomponent_3))
          (Default|UpdateDialogue (Variables|/Game/Blueprints/Gameplay/BP_Pawn.BP_Pawn_C|GetWBP_Dialogue Pawn) _charactername _dialoguelong_2))))))

(fn ConstructionScript
  (|CallParentFunction))