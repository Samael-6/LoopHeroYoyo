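; Player pawn for a dice-driven board game, moving between cells and triggering each cell's behavior through Activate and Update.
; StartPlay, meant to be called by the game mode once variables are set, creates the game and dialogue UI, then places the pawn and activates its cell.
; TryMoving asks Board for the destination, stores it in the GameInstance, then teleports and activates.
; A separate MoveNextCell event uses AIMoveTo without updating that index.
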(event Custom|MoveNextCell
  (params (DiceValue :type Integer))
  (Variables|Default|SetDeplacementNumber DiceValue)
  (Variables|Default|SetIsMoving true)
  (bind _cell (Default|GetCellbyNumber (Variables|Default|GetBoard) (Variables|/Game/Blueprints/Global/BP_LoopGameInstance.BP_LoopGameInstance_C|GetCellNumber (Variables|Default|GetBP_LoopGameInstance))))
  (AI|AIMoveTo self "0, 0, 0" 0 5.0 false
    (:then
      (Transformation|SetActorRotation (.rotation (Transformation|GetActorTransform _cell))))))

(event Custom|StartPlay
  (params (IsIntro :type Boolean))
  (bind _asbp_loop_game_instance (Utilities|Casting|CastToBP_LoopGameInstance (Game|GetGameInstance)))
  (Variables|Default|SetBP_LoopGameInstance _asbp_loop_game_instance)
  (bind _returnvalue (UserInterface|CreateWidget "/Game/Blueprints/HUD/WBP_UIGame.WBP_UIGame_C"))
  (bind _output_get (Variables|Default|SetWBP_UIGame _returnvalue))
  (UserInterface|Viewport|AddtoViewport _output_get 0)
  (CallFunction|MovetoCell)
  (bind _returnvalue_2 (UserInterface|CreateWidget "/Game/Blueprints/HUD/WBP_DialogueUI.WBP_DialogueUI_C"))
  (bind _output_get_2 (Variables|Default|SetWBP_Dialogue _returnvalue_2))
  (Variables|/Game/Blueprints/HUD/WBP_DialogueUI.WBP_DialogueUI_C|SetDice _output_get_2 (Variables|Default|GetDice))
  (Variables|/Game/Blueprints/HUD/WBP_DialogueUI.WBP_DialogueUI_C|SetPawn _output_get_2 self)
  (UserInterface|Viewport|AddtoViewport _output_get_2 0)
  (CallFunction|ActivateCell))

(event Collision|EventActorBeginOverlap
  (params (OtherActor :type Actor%20Object%20Reference)))

(event EventTick
  (params (DeltaSeconds :type Float%20%28single-precision%29))
  (if (and (not (Variables|Default|GetIsMoving)) (Variables|Default|GetIsMoving))
    _))

(fn ConstructionScript)

(fn MovetoCell
  (bind _cell (Default|GetCellbyNumber (Variables|Default|GetBoard) (Variables|/Game/Blueprints/Global/BP_LoopGameInstance.BP_LoopGameInstance_C|GetCellNumber (Variables|Default|GetBP_LoopGameInstance))))
  (Transformation|SetActorLocation (.location (Transformation|GetActorTransform _cell)) false false)
  (Transformation|SetActorRotation (.rotation (Transformation|GetActorTransform _cell))))

(fn TryMoving
  (params (ValueDice :type Integer))
  (bind _bp_loopgameinstance (Variables|Default|GetBP_LoopGameInstance))
  (bind _cell (Default|GetNextCelltoMove (Variables|Default|GetBoard) (+ ValueDice (Variables|/Game/Blueprints/Global/BP_LoopGameInstance.BP_LoopGameInstance_C|GetCellNumber _bp_loopgameinstance))))
  (Variables|/Game/Blueprints/Global/BP_LoopGameInstance.BP_LoopGameInstance_C|SetCellNumber _bp_loopgameinstance _cell)
  (CallFunction|MovetoCell)
  (CallFunction|ActivateCell))

(fn ActivateCell
  (bind _cell (Default|GetCellbyNumber (Variables|Default|GetBoard) (Variables|/Game/Blueprints/Global/BP_LoopGameInstance.BP_LoopGameInstance_C|GetCellNumber (Variables|Default|GetBP_LoopGameInstance))))
  (Default|Activate _cell self))

(fn UpdateCell
  (bind _cell (Default|GetCellbyNumber (Variables|Default|GetBoard) (Variables|/Game/Blueprints/Global/BP_LoopGameInstance.BP_LoopGameInstance_C|GetCellNumber (Variables|Default|GetBP_LoopGameInstance))))
  (Default|Update _cell self))