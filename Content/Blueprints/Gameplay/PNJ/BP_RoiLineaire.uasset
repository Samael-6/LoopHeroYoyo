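; BP_RoiLineaire is an NPC that runs a row-based dialogue and ends the game once the Sentinelle is defeated.
; Activate picks the victory row if the game instance flags that defeat, then feeds the dialogue component's current row into the pawn's dialogue widget.
; Update advances rows until the dialogue finishes, then closes it and either shows the win widget and quits after a delay, or resets to a repeat row.
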(event EventBeginPlay
  (|CallParentFunction)
  (bind _asbp_loop_game_instance (Utilities|Casting|CastToBP_LoopGameInstance (Game|GetGameInstance)))
  (Variables|Default|SetBP%20Loop%20Game%20Instance _asbp_loop_game_instance))

(event EventActivate
  (params (Pawn :type BP%20Pawn%20Object%20Reference))
  (bind _wbp_dialogue (Variables|/Game/Blueprints/Gameplay/BP_Pawn.BP_Pawn_C|GetWBP_Dialogue Pawn))
  (bind _bpc_dialoguecomponent (Variables|Default|GetBPC_DialogueComponent))
  (if (Variables|/Game/Blueprints/Global/BP_LoopGameInstance.BP_LoopGameInstance_C|GetIsSentinelleDefeated (Variables|Default|GetBP%20Loop%20Game%20Instance))
    (Variables|/Game/Blueprints/Global/BPC_DialogueComponent.BPC_DialogueComponent_C|SetCurrentRowNumber (Variables|Default|GetBPC_DialogueComponent) 14))
  (Default|GetCurrentDialogueRowData _bpc_dialoguecomponent)
  (bind _charactername (Default|GetCharacterfromCurrentRow _bpc_dialoguecomponent))
  (bind _dialoguelong (Default|GetDialogueLongfromCurrentRow _bpc_dialoguecomponent))
  (Default|UpdateDialogue _wbp_dialogue _charactername _dialoguelong)
  (Default|StartDialogue _wbp_dialogue (Variables|/Game/Blueprints/Gameplay/BP_Pawn.BP_Pawn_C|GetDice Pawn)))

(event EventUpdate
  (params (Pawn :type BP%20Pawn%20Object%20Reference))
  (bind _bpc_dialoguecomponent (Variables|Default|GetBPC_DialogueComponent))
  (bind _isdialoguefinished (Default|IsDialogueFinished (Variables|Default|GetBPC_DialogueComponent)))
  (if _isdialoguefinished
    (Default|ExitDialogue (Variables|/Game/Blueprints/Gameplay/BP_Pawn.BP_Pawn_C|GetWBP_Dialogue Pawn))
    (if (Variables|/Game/Blueprints/Global/BP_LoopGameInstance.BP_LoopGameInstance_C|GetIsSentinelleDefeated (Variables|Default|GetBP%20Loop%20Game%20Instance))
      (bind _returnvalue (UserInterface|CreateWidget "/Game/Blueprints/HUD/WBP_Win.WBP_Win_C"))
      (UserInterface|Viewport|AddtoViewport _returnvalue 0)
      (Utilities|FlowControl|Delay 3.0)
      (Game|QuitGame 0 "Quit" false)
      (else
        (Variables|/Game/Blueprints/Global/BPC_DialogueComponent.BPC_DialogueComponent_C|SetCurrentRowNumber (Variables|Default|GetBPC_DialogueComponent) 11)))
    (else
      (Default|ReadNextRow _bpc_dialoguecomponent)
      (bind _charactername (Default|GetCharacterfromCurrentRow _bpc_dialoguecomponent))
      (bind _dialoguelong (Default|GetDialogueLongfromCurrentRow _bpc_dialoguecomponent))
      (Default|UpdateDialogue (Variables|/Game/Blueprints/Gameplay/BP_Pawn.BP_Pawn_C|GetWBP_Dialogue Pawn) _charactername _dialoguelong))))

(fn ConstructionScript
  (|CallParentFunction))